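; BP_PawnTurret is a turret pawn that takes damage from projectiles and shows its health in a world widget.
; On BeginPlay it hands itself to the Health widget as owner, and each tick it rotates the widget component to face the player pawn.
; Hits from ProjectileBase actors on the turret mesh, base mesh or capsule each lower Health and raise Score by a fixed amount.
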(event `self.ReceiveBeginPlay`
  (bind _ashealth (cast `/Game/Blueprints/Health` (`WidgetComponent.GetUserWidgetObject` (`self.Widget`))))
  (set `/Game/Blueprints/Health.Owner` self _ashealth))

(event `self.ReceiveTick`
  (params (DeltaSeconds :type "Float (single-precision)"))
  (bind _widget (`self.Widget`))
  (`SceneComponent.K2_SetWorldRotation` _widget (`KismetMathLibrary.FindLookAtRotation` (`SceneComponent.K2_GetComponentLocation` _widget) (`self.K2_GetActorLocation` (`GameplayStatics.GetPlayerPawn` 0))) false false))

(event `self.TurretMesh.OnComponentHit`
  (params (HitComponent :type "PrimitiveComponent Object Reference") (OtherActor :type "Actor Object Reference") (OtherComp :type "PrimitiveComponent Object Reference") (NormalImpulse :type "Vector Structure") (Hit :type "HitResult Structure (by ref)"))
  (cast `ProjectileBase` OtherActor)
  (set `self.Health` (- (`self.Health`) 20.0))
  (set `self.Score` (+ (`self.Score`) 20.0)))

(event `self.BaseMesh.OnComponentHit`
  (params (HitComponent :type "PrimitiveComponent Object Reference") (OtherActor :type "Actor Object Reference") (OtherComp :type "PrimitiveComponent Object Reference") (NormalImpulse :type "Vector Structure") (Hit :type "HitResult Structure (by ref)"))
  (cast `ProjectileBase` OtherActor)
  (set `self.Health` (- (`self.Health`) 20.0))
  (set `self.Score` (+ (`self.Score`) 20.0)))

(event `self.CapsuleComp.OnComponentHit`
  (params (HitComponent :type "PrimitiveComponent Object Reference") (OtherActor :type "Actor Object Reference") (OtherComp :type "PrimitiveComponent Object Reference") (NormalImpulse :type "Vector Structure") (Hit :type "HitResult Structure (by ref)"))
  (cast `ProjectileBase` OtherActor)
  (set `self.Health` (- (`self.Health`) 20.0))
  (set `self.Score` (+ (`self.Score`) 20.0)))

(fn `UserConstructionScript`)